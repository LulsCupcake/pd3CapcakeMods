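; Bag selector station that cycles through 25 entries in a bag class list via plus and minus interactables, starting on BeginPlay.
; Each selection spawns that actor with interaction enabled, starts a new SBZBagSpawner using its bag type, and displays the type as text.
; Switching destroys the previous actor and every SBZBagItem in the world, but not earlier spawners.
; Unconnected leftover nodes cover cop duplication and asset scanning.
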(event `self.ReceiveBeginPlay`
  (bind _output (`|GetArrayItem` (`self.Bags`) (`self.CurrentBag`)))
  (bind _returnvalue (`|SpawnActorFromClass` _output (`SceneComponent.K2_GetComponentToWorld` (`self.Mesh`)) "Undefined" "OverrideRootScale" null null :!label _label))
  (`SBZSingleBagGenerator.SetInteractionEnabled` _returnvalue true)
  (bind _returnvalue_2 (`|SpawnActorFromClass` "/Script/Starbreeze.SBZBagSpawner" (`SceneComponent.K2_GetComponentToWorld` (`self.Bag`)) "Undefined" "OverrideRootScale" null null))
  (bind _output_get (set `SBZBagSpawner.BagTypeToSpawn` (`SBZSingleBagGenerator.BagType` (`LowEntryExtendedStandardLibrary.CreateObject` _output)) _returnvalue_2))
  (`SBZBagSpawner.StartSpawningBags` _returnvalue_2)
  (`TextRenderComponent.K2_SetText` (`self.TextRender`) (`KismetTextLibrary.Conv_ObjectToText` _output_get)))

(event `self.SBZInteractablePlus.OnEndInteraction`
  (params (Interactable :type "SBZBaseInteractableComponent Object Reference") (Interactor :type "SBZInteractorComponent Object Reference") (bIsLocallyControlledInteractor :type Boolean))
  (bind _output_get (set `self.CurrentBag` (+ (`self.CurrentBag`) 1)))
  (if (== _output_get 25)
    (set `self.CurrentBag` 0))
  (`self.K2_DestroyActor` (stale `self.ReceiveBeginPlay` _returnvalue) :!label _label_2)
  (bind _outactors (`GameplayStatics.GetAllActorsOfClass` "/Script/Starbreeze.SBZBagItem"))
  (for _array_element _outactors
    (`self.K2_DestroyActor` _array_element))
  (goto _label))

(event `self.SBZInteractableMinus.OnEndInteraction`
  (params (Interactable :type "SBZBaseInteractableComponent Object Reference") (Interactor :type "SBZInteractorComponent Object Reference") (bIsLocallyControlledInteractor :type Boolean))
  (bind _output_get (set `self.CurrentBag` (+ (`self.CurrentBag`) -1)))
  (if (== _output_get -1)
    (set `self.CurrentBag` 24)
    (goto _label_2)
    (else
      (goto _label_2))))

(fn `UserConstructionScript`)