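; Level changer Blueprint in the EnemySpawner mod that streams sets of map sublevels in and out through custom events.
; LoadPG_Event and UnloadPG_Event load and unload the tutorial warehouse, combat architecture, props, lighting and PGUnits levels, non-blocking via soft object references.
; ArmouredTransport_Event streams in the ArmoredTransport level, then calls ScanFilesSynchronousMessage without forcing a rescan, and has no matching unload event.
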(event `UnloadPG_Event`
  (`GameplayStatics.UnloadStreamLevelBySoftObjectPtr` "/Game/Prototype/Maps/Tutorial/_common/E_Tutorial_Warehouse.E_Tutorial_Warehouse")
  (`GameplayStatics.UnloadStreamLevelBySoftObjectPtr` "/Game/Prototype/Maps/Tutorial/Loud/LoudTutCombat/Sublevels/Environment_LoudTutCombat/E_LoudTutCombat_Arch.E_LoudTutCombat_Arch")
  (`GameplayStatics.UnloadStreamLevelBySoftObjectPtr` "/Game/Prototype/Maps/Tutorial/Loud/LoudTutCombat/Sublevels/Environment_LoudTutCombat/E_LoudTutCombat_Prop.E_LoudTutCombat_Prop")
  (`GameplayStatics.UnloadStreamLevelBySoftObjectPtr` "/Game/Mods/_CapcakeMods/EnemySpawner/Levels/PGUnits.PGUnits")
  (`GameplayStatics.UnloadStreamLevelBySoftObjectPtr` "/Game/Prototype/Maps/Tutorial/Loud/LoudTutCombat/Sublevels/Lighting_LoudTutCombat/L_LoudTutCombat_Lighting.L_LoudTutCombat_Lighting"))

(event `LoadPG_Event`
  (`GameplayStatics.LoadStreamLevelBySoftObjectPtr` "/Game/Prototype/Maps/Tutorial/Loud/LoudTutCombat/Sublevels/Environment_LoudTutCombat/E_LoudTutCombat_Arch.E_LoudTutCombat_Arch" true)
  (`GameplayStatics.LoadStreamLevelBySoftObjectPtr` "/Game/Prototype/Maps/Tutorial/Loud/LoudTutCombat/Sublevels/Environment_LoudTutCombat/E_LoudTutCombat_Prop.E_LoudTutCombat_Prop" true)
  (`GameplayStatics.LoadStreamLevelBySoftObjectPtr` "/Game/Prototype/Maps/Tutorial/_common/E_Tutorial_Warehouse.E_Tutorial_Warehouse" true)
  (`GameplayStatics.LoadStreamLevelBySoftObjectPtr` "/Game/Mods/_CapcakeMods/EnemySpawner/Levels/PGUnits.PGUnits" true)
  (`GameplayStatics.LoadStreamLevelBySoftObjectPtr` "/Game/Prototype/Maps/Tutorial/Loud/LoudTutCombat/Sublevels/Lighting_LoudTutCombat/L_LoudTutCombat_Lighting.L_LoudTutCombat_Lighting" true))

(event `ArmouredTransport_Event`
  (`GameplayStatics.LoadStreamLevelBySoftObjectPtr` "/Game/Prototype/Maps/ArmouredTransport/ArmoredTransport.ArmoredTransport" true)
  (message `AssetRegistry.ScanFilesSynchronous` _))

(fn `UserConstructionScript`)