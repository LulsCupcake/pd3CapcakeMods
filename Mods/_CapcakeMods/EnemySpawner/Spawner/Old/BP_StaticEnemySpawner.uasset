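; Old static enemy spawner Blueprint from a mod; the logic shown spawns nothing and only spins an AI character.
; BeginPlay binds an empty overlap handler on AIVolume, whose OverlappedActor output Tick casts to SBZAICharacter and yaws slightly each frame while IsSpinning is set.
; ToggleSpin flip-flops that flag, setting it false on the first call.
; A static mesh rotation node is left unconnected.
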(event `self.ReceiveBeginPlay`
  (add `self.OnActorBeginOverlap` (`self.AIVolume`) (delegate `OnActorBeginOverlap_Event_0`)))

(event `OnActorBeginOverlap_Event_0` :!signature `self.OnActorBeginOverlap`
  (params (OverlappedActor :type "Actor Object Reference") (OtherActor :type "Actor Object Reference")))

(event `self.ReceiveTick`
  (params (DeltaSeconds :type "Float (single-precision)"))
  (if (`self.IsSpinning`)
    (bind _assbzaicharacter (cast `SBZAICharacter` (stale `OnActorBeginOverlap_Event_0` OverlappedActor)))
    (`self.K2_AddActorWorldRotation` _assbzaicharacter (struct :`Yaw` 0.4) false false)))

(event `ToggleSpin`
  (`/Engine/EditorBlueprintResources/StandardMacros.FlipFlop`
    (:`A`
      (set `self.IsSpinning` false))
    (:`B`
      (set `self.IsSpinning` true))))

(fn `UserConstructionScript`)