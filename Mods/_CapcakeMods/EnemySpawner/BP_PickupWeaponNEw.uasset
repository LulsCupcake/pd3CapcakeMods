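; Interactable weapon pickup actor in a mod that alternates its stored weapon config each time it is used.
; Interaction is enabled on BeginPlay, and each server-side completion drives a FlipFlop that sets StoredWeaponConfig to an empty config or the Commando SMG, starting with empty.
; After a short delay the interaction is re-enabled for reuse.
; The graph only stores the config and contains no logic to give the weapon to a player.
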(event `self.ReceiveBeginPlay`
  (`SBZInteractableComponent.SetInteractionEnabled` (`self.Interactable`) true))

(event `self.Interactable.OnServerCompleteInteraction`
  (params (Interactable :type "SBZBaseInteractableComponent Object Reference") (Interactor :type "SBZInteractorComponent Object Reference") (bIsLocallyControlledInteractor :type Boolean))
  (`/Engine/EditorBlueprintResources/StandardMacros.FlipFlop`
    (:`A`
      (set `SBZPlaceableWeapon.StoredWeaponConfig` (make `SBZEquippableConfig` null)))
    (:`B`
      (set `SBZPlaceableWeapon.StoredWeaponConfig` (make `SBZEquippableConfig` "/Game/Gameplay/Weapons/SMG/Commando/DA_WeaponData_SMG_Commando.DA_WeaponData_SMG_Commando"))))
  (`KismetSystemLibrary.Delay` 1.0)
  (`SBZInteractableComponent.SetInteractionEnabled` (`self.Interactable`) true))

(fn `UserConstructionScript`)