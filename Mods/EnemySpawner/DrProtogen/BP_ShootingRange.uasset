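; Shooting range test actor that displays last and total damage, plus the damage type, instigator and causer of each hit.
; One interactable cycles how those objects are named (path, display, object or class name), and another resets the damage totals.
; A range interactable steps the hitbox through preset distances from 1 to 50 meters via a looping MultiGate and timeline lerp.
; The startfix event runs the range and naming logic to initialize the displays.
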(event `self.ReceiveAnyDamage`
  (params (Damage :type "Float (single-precision)") (DamageType :type "DamageType Object Reference") (InstigatedBy :type "Controller Object Reference") (DamageCauser :type "Actor Object Reference"))
  (bind _output_get (set `self.Damage` Damage))
  (`TextRenderComponent.K2_SetText` (`self.DamageText`) (`KismetTextLibrary.Conv_DoubleToText` _output_get "HalfToEven"))
  (bind _output_get_2 (set `self.TotalDamage` (+ _output_get (`self.TotalDamage`))))
  (`TextRenderComponent.K2_SetText` (`self.TotalDamageText`) (`KismetTextLibrary.Conv_DoubleToText` _output_get_2 "HalfToEven"))
  (if (== (`self.State`) 0)
    (`TextRenderComponent.K2_SetText` (`self.DamageType`) (`KismetTextLibrary.Conv_StringToText` (`KismetSystemLibrary.GetPathName` DamageType)))
    (`TextRenderComponent.K2_SetText` (`self.Instigated`) (`KismetTextLibrary.Conv_StringToText` (`KismetSystemLibrary.GetPathName` InstigatedBy)))
    (`TextRenderComponent.K2_SetText` (`self.CauseOfDamage`) (`KismetTextLibrary.Conv_StringToText` (`KismetSystemLibrary.GetPathName` DamageCauser)))
    (elif (== (`self.State`) 1)
      (`TextRenderComponent.K2_SetText` (`self.DamageType`) (`KismetTextLibrary.Conv_StringToText` (`KismetSystemLibrary.GetDisplayName` DamageType)))
      (`TextRenderComponent.K2_SetText` (`self.Instigated`) (`KismetTextLibrary.Conv_StringToText` (`KismetSystemLibrary.GetDisplayName` InstigatedBy)))
      (`TextRenderComponent.K2_SetText` (`self.CauseOfDamage`) (`KismetTextLibrary.Conv_StringToText` (`KismetSystemLibrary.GetDisplayName` DamageCauser)))
      (elif (== (`self.State`) 2)
        (`TextRenderComponent.K2_SetText` (`self.DamageType`) (`KismetTextLibrary.Conv_StringToText` (`KismetSystemLibrary.GetObjectName` DamageType)))
        (`TextRenderComponent.K2_SetText` (`self.Instigated`) (`KismetTextLibrary.Conv_StringToText` (`KismetSystemLibrary.GetObjectName` InstigatedBy)))
        (`TextRenderComponent.K2_SetText` (`self.CauseOfDamage`) (`KismetTextLibrary.Conv_StringToText` (`KismetSystemLibrary.GetObjectName` DamageCauser)))
        (elif (== (`self.State`) 3)
          (`TextRenderComponent.K2_SetText` (`self.DamageType`) (`KismetTextLibrary.Conv_StringToText` (`KismetSystemLibrary.GetClassDisplayName` (`GameplayStatics.GetObjectClass` DamageCauser))))
          (`TextRenderComponent.K2_SetText` (`self.Instigated`) (`KismetTextLibrary.Conv_StringToText` (`KismetSystemLibrary.GetClassDisplayName` (`GameplayStatics.GetObjectClass` InstigatedBy))))
          (`TextRenderComponent.K2_SetText` (`self.CauseOfDamage`) (`KismetTextLibrary.Conv_StringToText` (`KismetSystemLibrary.GetClassDisplayName` (`GameplayStatics.GetObjectClass` DamageType)))))))))

(event `self.SBZInteractableSetting.OnServerCompleteInteraction`
  (params (Interactable :type "SBZBaseInteractableComponent Object Reference") (Interactor :type "SBZInteractorComponent Object Reference") (bIsLocallyControlledInteractor :type Boolean))
  (if (== (`self.State`) 0) :!label _label
    (set `self.State` 1)
    (`TextRenderComponent.K2_SetText` (`self.Current State`) (stale _output_get))
    (bind _output_get (set `self.TextData` "Getting Display Name"))
    (elif (== (`self.State`) 1)
      (set `self.State` 2)
      (`TextRenderComponent.K2_SetText` (`self.Current State`) (stale _output_get_2))
      (bind _output_get_2 (set `self.TextData` "Getting Object Name"))
      (elif (== (`self.State`) 2)
        (set `self.State` 3)
        (`TextRenderComponent.K2_SetText` (`self.Current State`) (stale _output_get_3))
        (bind _output_get_3 (set `self.TextData` "Getting Class Name"))
        (elif (== (`self.State`) 3)
          (set `self.State` 0)
          (`TextRenderComponent.K2_SetText` (`self.Current State`) (stale _output_get_4) :!label _label_2)
          (bind _output_get_4 (set `self.TextData` "Getting Path Name")))))))

(event `startfix`
  (`|ExecutionSequence`
    (:`then_0`
      (`|MultiGate` false true 0 :!label _label_3
        (:`Out 0`
          (set `self.CurrentRange` 1)
          (set `self.NewLocation` (3015.0 -1437.0 130.0)))
        (:`Out 1`
          (set `self.CurrentRange` 5)
          (set `self.NewLocation` (3415.0 -1437.0 130.0)))
        (:`Out 2`
          (set `self.CurrentRange` 10)
          (set `self.NewLocation` (3915.0 -1437.0 130.0)))
        (:`Out 3`
          (set `self.CurrentRange` 20)
          (set `self.NewLocation` (4915.0 -1437.0 130.0)))
        (:`Out 4`
          (set `self.CurrentRange` 30)
          (set `self.NewLocation` (5915.0 -1437.0 130.0)))
        (:`Out 5`
          (set `self.CurrentRange` 40)
          (set `self.NewLocation` (6915.0 -1437.0 130.0)))
        (:`Out 6`
          (set `self.CurrentRange` 50)
          (set `self.NewLocation` (7915.0 -1437.0 130.0))))
      (`TextRenderComponent.K2_SetText` (`self.Range`) (`KismetTextLibrary.Conv_StringToText` (`KismetStringLibrary.Concat_StrStr` (`KismetStringLibrary.Conv_IntToString` (`self.CurrentRange`)) " meters")))
      (bind (_direction _lerp0_1) (`Timeline|Timeline_0` :!via `PlayFromStart`)
        (:`Update`
          (`SceneComponent.K2_SetWorldLocation` (`self.Hitbox`) (`KismetMathLibrary.VLerp` (`SceneComponent.K2_GetComponentLocation` (`self.Hitbox`)) (`self.NewLocation`) _lerp0_1) false false))
        (:`Finished`
          (`SBZInteractableComponent.SetInteractionEnabled` (`self.SBZInteractableRange`) true))))
    (:`then_1`
      (goto _label))
    (:`then_2`
      (goto _label_2))))

(event `self.SBZInteractableDamage.OnServerCompleteInteraction`
  (params (Interactable :type "SBZBaseInteractableComponent Object Reference") (Interactor :type "SBZInteractorComponent Object Reference") (bIsLocallyControlledInteractor :type Boolean))
  (set `self.TotalDamage` 0.0)
  (set `self.Damage` 0.0)
  (bind _output_get (set `self.DamagePerSecond` 0.0))
  (`TextRenderComponent.K2_SetText` (`self.DamageText`) (`KismetTextLibrary.Conv_DoubleToText` _output_get "HalfToEven"))
  (`TextRenderComponent.K2_SetText` (`self.TotalDamageText`) (`KismetTextLibrary.Conv_DoubleToText` _output_get "HalfToEven")))

(event `self.SBZInteractableRange.OnServerEndInteraction`
  (params (Interactable :type "SBZBaseInteractableComponent Object Reference") (Interactor :type "SBZInteractorComponent Object Reference") (bIsLocallyControlledInteractor :type Boolean))
  (goto _label_3))

(fn `UserConstructionScript`)