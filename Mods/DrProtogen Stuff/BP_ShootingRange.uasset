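; BP_ShootingRange is a damage-testing target that shows the last hit, running total, damage type, instigator and causer on text components.
; One interactable cycles how those objects are named (path, display, object or class name); its mode label updates before TextData changes, so lags a step.
; Class mode swaps the damage type and causer fields.
; A second interactable zeroes the damage readouts; DamagePerSecond is only reset, never calculated.
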(event `self.ReceiveBeginPlay`
  (set `self.State` 0)
  (`TextRenderComponent.K2_SetText` (`self.DamageType`) (`KismetTextLibrary.Conv_StringToText` (`KismetSystemLibrary.GetPathName` (stale `self.ReceiveAnyDamage` DamageType))))
  (`TextRenderComponent.K2_SetText` (`self.Instigated`) (`KismetTextLibrary.Conv_StringToText` (`KismetSystemLibrary.GetPathName` (stale `self.ReceiveAnyDamage` InstigatedBy))))
  (`TextRenderComponent.K2_SetText` (`self.CauseOfDamage`) (`KismetTextLibrary.Conv_StringToText` (`KismetSystemLibrary.GetPathName` (stale `self.ReceiveAnyDamage` DamageCauser))))
  (bind _output_get (set `self.TextData` "Getting Path Name"))
  (`TextRenderComponent.K2_SetText` (`self.Current State`) _output_get))

(event `self.ReceiveAnyDamage`
  (params (Damage :type "Float (single-precision)") (DamageType :type "DamageType Object Reference") (InstigatedBy :type "Controller Object Reference") (DamageCauser :type "Actor Object Reference"))
  (bind _output_get (set `self.Damage` Damage))
  (`TextRenderComponent.K2_SetText` (`self.DamageText`) (`KismetTextLibrary.Conv_DoubleToText` _output_get "HalfToEven"))
  (bind _output_get_2 (set `self.TotalDamage` (+ _output_get (`self.TotalDamage`))))
  (`TextRenderComponent.K2_SetText` (`self.TotalDamageText`) (`KismetTextLibrary.Conv_DoubleToText` _output_get_2 "HalfToEven"))
  (if (== (`self.State`) 0)
    (`TextRenderComponent.K2_SetText` (`self.DamageType`) (`KismetTextLibrary.Conv_StringToText` (`KismetSystemLibrary.GetPathName` DamageType)))
    (`TextRenderComponent.K2_SetText` (`self.Instigated`) (`KismetTextLibrary.Conv_StringToText` (`KismetSystemLibrary.GetPathName` InstigatedBy)))
    (`TextRenderComponent.K2_SetText` (`self.CauseOfDamage`) (`KismetTextLibrary.Conv_StringToText` (`KismetSystemLibrary.GetPathName` DamageCauser)))
    (elif (== (`self.State`) 1)
      (`TextRenderComponent.K2_SetText` (`self.DamageType`) (`KismetTextLibrary.Conv_StringToText` (`KismetSystemLibrary.GetDisplayName` DamageType)))
      (`TextRenderComponent.K2_SetText` (`self.Instigated`) (`KismetTextLibrary.Conv_StringToText` (`KismetSystemLibrary.GetDisplayName` InstigatedBy)))
      (`TextRenderComponent.K2_SetText` (`self.CauseOfDamage`) (`KismetTextLibrary.Conv_StringToText` (`KismetSystemLibrary.GetDisplayName` DamageCauser)))
      (elif (== (`self.State`) 2)
        (`TextRenderComponent.K2_SetText` (`self.DamageType`) (`KismetTextLibrary.Conv_StringToText` (`KismetSystemLibrary.GetObjectName` DamageType)))
        (`TextRenderComponent.K2_SetText` (`self.Instigated`) (`KismetTextLibrary.Conv_StringToText` (`KismetSystemLibrary.GetObjectName` InstigatedBy)))
        (`TextRenderComponent.K2_SetText` (`self.CauseOfDamage`) (`KismetTextLibrary.Conv_StringToText` (`KismetSystemLibrary.GetObjectName` DamageCauser)))
        (elif (== (`self.State`) 3)
          (`TextRenderComponent.K2_SetText` (`self.DamageType`) (`KismetTextLibrary.Conv_StringToText` (`KismetSystemLibrary.GetClassDisplayName` (`GameplayStatics.GetObjectClass` DamageCauser))))
          (`TextRenderComponent.K2_SetText` (`self.Instigated`) (`KismetTextLibrary.Conv_StringToText` (`KismetSystemLibrary.GetClassDisplayName` (`GameplayStatics.GetObjectClass` InstigatedBy))))
          (`TextRenderComponent.K2_SetText` (`self.CauseOfDamage`) (`KismetTextLibrary.Conv_StringToText` (`KismetSystemLibrary.GetClassDisplayName` (`GameplayStatics.GetObjectClass` DamageType)))))))))

(event `self.SBZInteractable.OnServerCompleteInteraction`
  (params (Interactable :type "SBZBaseInteractableComponent Object Reference") (Interactor :type "SBZInteractorComponent Object Reference") (bIsLocallyControlledInteractor :type Boolean))
  (if (== (`self.State`) 0)
    (set `self.State` 1)
    (`TextRenderComponent.K2_SetText` (`self.Current State`) (stale _output_get))
    (bind _output_get (set `self.TextData` "Getting Display Name"))
    (elif (== (`self.State`) 1)
      (set `self.State` 2)
      (`TextRenderComponent.K2_SetText` (`self.Current State`) (stale _output_get_2))
      (bind _output_get_2 (set `self.TextData` "Getting Object Name"))
      (elif (== (`self.State`) 2)
        (set `self.State` 3)
        (`TextRenderComponent.K2_SetText` (`self.Current State`) (stale _output_get_3))
        (bind _output_get_3 (set `self.TextData` "Getting Class Name"))
        (elif (== (`self.State`) 3)
          (set `self.State` 0)
          (`TextRenderComponent.K2_SetText` (`self.Current State`) (stale _output_get_4))
          (bind _output_get_4 (set `self.TextData` "Getting Path Name")))))))

(event `self.SBZInteractable1.OnServerCompleteInteraction`
  (params (Interactable :type "SBZBaseInteractableComponent Object Reference") (Interactor :type "SBZInteractorComponent Object Reference") (bIsLocallyControlledInteractor :type Boolean))
  (set `self.TotalDamage` 0.0)
  (set `self.Damage` 0.0)
  (bind _output_get (set `self.DamagePerSecond` 0.0))
  (`TextRenderComponent.K2_SetText` (`self.DamageText`) (`KismetTextLibrary.Conv_DoubleToText` _output_get "HalfToEven"))
  (`TextRenderComponent.K2_SetText` (`self.TotalDamageText`) (`KismetTextLibrary.Conv_DoubleToText` _output_get "HalfToEven")))

(fn `UserConstructionScript`)